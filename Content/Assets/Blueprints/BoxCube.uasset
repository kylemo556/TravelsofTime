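; BoxCube is a box the side-scroller character can push and pull, with a rewind to its starting transform.
; BeginPlay stores location and rotation, which R restores before detaching the box.
; InteractArea overlaps set InRange, letting Space toggle attachment to the character after a small offset scaled by its forward vector.
; The cube's physics constraint switches to the YZ plane for grabbing and back to default on release.
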(event `Key|R`
  (params (Key :type "Key Structure" :default "AnyKey"))
  ;[1 1 1] Rewind (Reset position & rotation)
  (:`Pressed`
    (`self.K2_SetActorLocation` (`self.startLoc`))
    (`self.SetActorRotation` (`self.startRot`))
    ;[1 1 1] Attach for push and pull
    (`self.DetachRootComponentFromParent` true :!label _label)
    (set `/Game/Assets/Blueprints/SideScrollerCharacter.Attached` false (`|ConvertAsset` (`self.character`)))
    (`PrimitiveComponent.SetConstraintMode` (`self.Cube`) "Default")))

(event `self.ReceiveBeginPlay`
  ;[1 1 1] Set Reset Location
  (set `self.startLoc` (`self.K2_GetActorLocation`))
  (set `self.startRot` (`self.K2_GetActorRotation`)))

(event `Key|SpaceBar`
  (params (Key :type "Key Structure" :default "AnyKey"))
  ;[1 1 1] Attach for push and pull
  (:`Pressed`
    (if (`self.inRange`)
      (`PrimitiveComponent.SetConstraintMode` (`self.Cube`) "YZPlane")
      (if (`/Game/Assets/Blueprints/SideScrollerCharacter.Attached` (`|ConvertAsset` (`self.character`)))
        (goto _label)
        (else
          (`SceneComponent.K2_AddLocalOffset` (`self.Cube`) (* (`self.GetActorForwardVector` (`|ConvertAsset` (`self.character`))) (0.0 10.0 0.0)) false false)
          (`self.K2_AttachRootComponentToActor` (`|ConvertAsset` (`self.character`)) "None" "KeepWorldPosition")
          (set `/Game/Assets/Blueprints/SideScrollerCharacter.Attached` true (`|ConvertAsset` (`self.character`))))))))

(event `self.InteractArea.OnComponentBeginOverlap`
  (params (OtherActor :type "Actor Object Reference") (OtherComp :type "PrimitiveComponent Object Reference") (OtherBodyIndex :type Integer) (bFromSweep :type Boolean) (SweepResult :type "HitResult Structure (by ref)"))
  ;[1 1 1] Checks if PC is in actor's push/pull range
  (cast `/Game/Assets/Blueprints/SideScrollerCharacter` OtherActor
    (:`then`
      (set `self.inRange` true :!label _label_2))
    (:`CastFailed`
      (set `self.inRange` false :!label _label_3))))

(event `self.InteractArea.OnComponentEndOverlap`
  (params (OtherActor :type "Actor Object Reference") (OtherComp :type "PrimitiveComponent Object Reference") (OtherBodyIndex :type Integer))
  ;[1 1 1] Checks if PC is in actor's push/pull range
  (cast `/Game/Assets/Blueprints/SideScrollerCharacter` OtherActor
    (:`then`
      (goto _label_3))
    (:`CastFailed`
      (goto _label_2))))

(fn `UserConstructionScript`)