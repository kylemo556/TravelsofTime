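; Torch actor whose bounce light and point light burn down over time and relight when the player presses R.
; BeginPlay stores the bounce light's starting intensity and enables player input.
; Tick lowers both lights by a fixed, frame-rate-dependent step while the bounce light stays above a floor, printing their intensities.
; R resets both lights to that single stored value.
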(event `Key|R`
  (params (Key :type "Key Structure" :default "AnyKey"))
  (bind _intensitystart (`self.IntensityStart`))
  (:`Pressed`
    (`LightComponent.SetIntensity` (`self.BounceLight`) _intensitystart)
    (`LightComponent.SetIntensity` (`self.PointLight`) _intensitystart)))

(event `self.ReceiveBeginPlay`
  (set `self.IntensityStart` (`LightComponentBase.Intensity` (`self.BounceLight`)))
  (`self.EnableInput` (`GameplayStatics.GetPlayerController` 0)))

(event `self.ReceiveTick`
  (params (DeltaSeconds :type "Float (single-precision)"))
  (bind _bouncelight (`self.BounceLight`))
  (bind _pointlight (`self.PointLight`))
  (bind _intensity (`LightComponentBase.Intensity` _pointlight))
  (bind _intensity_2 (`LightComponentBase.Intensity` _bouncelight))
  (if (> _intensity_2 1000.0)
    (`LightComponent.SetIntensity` _bouncelight (- _intensity_2 50.0))
    (`LightComponent.SetIntensity` _pointlight (- _intensity 50.0))
    (`KismetSystemLibrary.PrintString` (`KismetStringLibrary.Conv_DoubleToString` _intensity_2))
    (`KismetSystemLibrary.PrintString` (`KismetStringLibrary.Conv_DoubleToString` _intensity))))

(fn `UserConstructionScript`)