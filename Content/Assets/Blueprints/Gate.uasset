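; Gate Blueprint with two door meshes that open and close according to a referenced Switch's Open state.
; BeginPlay caches the world start location of each door.
; Every Tick it polls the switch and snaps the doors either apart along the world X axis or back to their start positions, with no interpolation or sweep.
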(event `self.ReceiveBeginPlay`
  ;[1 1 1] Save inital state
  (set `self.DoorLStart` (`SceneComponent.K2_GetComponentLocation` (`self.DoorL`)))
  (set `self.DoorRStart` (`SceneComponent.K2_GetComponentLocation` (`self.DoorR`))))

(event `self.ReceiveTick`
  (params (DeltaSeconds :type "Float (single-precision)"))
  ;[1 1 1] Change gate state on switch
  (if (`/Game/Assets/Blueprints/Switch.Open` (`self.Switch`))
    (`SceneComponent.K2_SetWorldLocation` (`self.DoorL`) (+ (`self.DoorLStart`) (-200.0 0.0 0.0)) false false)
    (`SceneComponent.K2_SetWorldLocation` (`self.DoorR`) (+ (`self.DoorRStart`) (200.0 0.0 0.0)) false false)
    (else
      (`SceneComponent.K2_SetWorldLocation` (`self.DoorL`) (`self.DoorLStart`) false false)
      (`SceneComponent.K2_SetWorldLocation` (`self.DoorR`) (`self.DoorRStart`) false false))))

(fn `UserConstructionScript`)